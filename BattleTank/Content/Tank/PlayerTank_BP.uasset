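; Player-controlled tank Blueprint that sets up its turret, barrel and track meshes, wires them into TankAiming and TankMovement components, and binds a health bar widget to itself.
; Input drives movement, gimbal and spring-arm camera rotation, firing with a sound, and first/third-person camera toggling.
; Tick runs a 200-second Delay, then opens the WinEnd level in UI-only input mode if only one Tank actor remains.
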(event `self.ReceiveBeginPlay`
  (`TankAimingComponent.Initialise` (`self.TankAiming`) (`self.Barrel`) (`self.Turret`))
  (`TankMovementComponent.Initialise` (`self.TankMovement`) (`self.TankTrack`) (`self.TankTrack1`))
  (`self.Initialize Health Bar Widget`))

(event `InputAction|Swap Cam`
  (params (Key :type "Key Structure"))
  (:`Pressed`
    (`ActorComponent.ToggleActive` (`self.1st Person`))
    (`ActorComponent.ToggleActive` (`self.3rd Person`))))

(event `InputAxis|AimH`
  (params (AxisValue :type "Float (single-precision)"))
  ;[1 1 1] Firing
  (`SceneComponent.K2_AddLocalRotation` (`self.H Gimbal`) (`KismetMathLibrary.MakeRotator` 0.0 0.0 (* AxisValue (`GameplayStatics.GetWorldDeltaSeconds`) 100.0)) false false))

(event `InputAxis|Move Forward`
  (params (AxisValue :type "Float (single-precision)"))
  ;[1 1 1] Movement
  (`TankMovementComponent.IntendMoveForwards` (`self.TankMovement`) AxisValue))

(event `InputAxis|Turn Right`
  (params (AxisValue :type "Float (single-precision)"))
  ;[1 1 1] Movement
  (`TankMovementComponent.IntendTurnRight` (`self.TankMovement`) AxisValue))

(event `InputAxis|AimV`
  (params (AxisValue :type "Float (single-precision)"))
  ;[1 1 1] Firing
  (`SceneComponent.K2_AddLocalRotation` (`self.SpringArm`) (`KismetMathLibrary.MakeRotator` 0.0 (* AxisValue (`GameplayStatics.GetWorldDeltaSeconds`) 100.0)) false false))

(event `InputAction|Fire`
  (params (Key :type "Key Structure"))
  ;[1 1 1] Firing
  (:`Pressed`
    (`GameplayStatics.PlaySound2D` "/Game/Sounds/Explosion01_Cue.Explosion01_Cue" 1.0 1.0 0.0 null null)
    (`TankAimingComponent.Fire` (`self.TankAiming`))))

(event `self.ReceiveTick`
  (params (DeltaSeconds :type "Float (single-precision)"))
  (`KismetSystemLibrary.Delay` 200.0)
  (bind _outactors (`GameplayStatics.GetAllActorsOfClass` "/Script/BattleTank.Tank"))
  (if (== (`KismetArrayLibrary.Array_Length` _outactors) 1)
    (`WidgetBlueprintLibrary.SetInputMode_UIOnlyEx` (`GameplayStatics.GetPlayerController` 0) null)
    (`GameplayStatics.OpenLevel` "WinEnd")))

(fn `Initialize Health Bar Widget`
  (bind _ashealth_bar (cast `/Game/UI/HealthBar` (`WidgetComponent.GetUserWidgetObject` (`self.Health Bar`))))
  (set `/Game/UI/HealthBar.Tank` self _ashealth_bar)
  (return))

(fn `UserConstructionScript`
  (`StaticMeshComponent.SetStaticMesh` (`self.Turret`) "/Game/Tank/tank_fbx_Turret.tank_fbx_Turret")
  (`StaticMeshComponent.SetStaticMesh` (`self.Barrel`) "/Game/Tank/tank_fbx_Barrel.tank_fbx_Barrel")
  (`StaticMeshComponent.SetStaticMesh` (`self.TankTrack`) "/Game/Tank/tank_fbx_Track.tank_fbx_Track")
  (`StaticMeshComponent.SetStaticMesh` (`self.TankTrack1`) "/Game/Tank/tank_fbx_Track.tank_fbx_Track")
  (`PrimitiveComponent.SetCollisionEnabled` (`self.Turret`) "NoCollision")
  (`PrimitiveComponent.SetCollisionEnabled` (`self.Barrel`) "NoCollision")
  (`PrimitiveComponent.SetEnableGravity` (`self.Turret`) false)
  (`PrimitiveComponent.SetEnableGravity` (`self.Barrel`) false))